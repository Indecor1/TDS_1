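; DoorBP is a sliding door that opens and closes as characters overlap its two trigger volumes.
; Overlapping EnterTrigger opens it and overlapping ExitTrigger closes it, with an IsOpen flag blocking repeat calls.
; The OpenDoor timeline drives the slum wall mesh's relative X location, playing from start to open and reversing from end to close.
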(event OnComponentBeginOverlap(ExitTrigger)
  (params (OverlappedComponent :type Primitive%20Component%20Object%20Reference) (OtherActor :type Actor%20Object%20Reference) (OtherComp :type Primitive%20Component%20Object%20Reference) (OtherBodyIndex :type Integer) (bFromSweep :type Boolean) (SweepResult :type Hit%20Result%20Structure%20%28by%20ref%29))
  (Utilities|Casting|CastToCharacter OtherActor)
  (CallFunction|Closing))

(event OnComponentBeginOverlap(EnterTrigger)
  (params (OverlappedComponent :type Primitive%20Component%20Object%20Reference) (OtherActor :type Actor%20Object%20Reference) (OtherComp :type Primitive%20Component%20Object%20Reference) (OtherBodyIndex :type Integer) (bFromSweep :type Boolean) (SweepResult :type Hit%20Result%20Structure%20%28by%20ref%29))
  (Utilities|Casting|CastToCharacter OtherActor)
  (CallFunction|Opening))

(event Custom|Closing
  (if (Variables|Default|GetIsOpen)
    (Variables|Default|SetIsOpen false)
    (bind _xoffset (Timeline|OpenDoor ReverseFromEnd)
      (:Update
        (Transformation|SetRelativeLocation (Variables|Default|GetSM_Slums_Wall_01d) (Math|Vector|MakeVector _xoffset 0.0 0.0) false false)))))

(event Custom|Opening
  (if (not (Variables|Default|GetIsOpen))
    (Variables|Default|SetIsOpen true)
    (bind _xoffset (Timeline|OpenDoor PlayFromStart)
      (:Update
        (Transformation|SetRelativeLocation (Variables|Default|GetSM_Slums_Wall_01d) (Math|Vector|MakeVector _xoffset 0.0 0.0) false false)))))

(event EventBeginPlay)

(event Collision|EventActorBeginOverlap
  (params (OtherActor :type Actor%20Object%20Reference)))

(event EventTick
  (params (DeltaSeconds :type Float%20%28single-precision%29)))

(fn ConstructionScript)